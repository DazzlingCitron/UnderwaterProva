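; BP_FlashController plays a timed sequence of screen flashes, then speeds up every manta ray in the level.
; Tick passes through a one-second Delay and a DoOnce into a countdown loop on LoopTimes.
; Each pass waits an interval from the Duration array, then adds a new W_FlashEffect widget to the viewport.
; When the count runs out, each BP_MantaRay's spline speed and Manta play rate are multiplied by SpeedUpFactor.
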(event EventBeginPlay)

(event Collision|EventActorBeginOverlap
  (params (OtherActor :type Actor%20Object%20Reference)))

(event EventTick
  (params (DeltaSeconds :type Float%20%28single-precision%29))
  (bind _speedupfactor (Variables|Default|GetSpeedUpFactor))
  (Utilities|FlowControl|Delay 1.0)
  ;[1 1 1] 5 Flashes
  (Utilities|FlowControl|DoOnce false
    (:Completed
      (if (> (Variables|Components|GetLoopTimes) 0) :!label _label
        (Utilities|FlowControl|Delay (Utilities|Array|Get(acopy) (Variables|Components|GetDuration) (- 5 (Variables|Components|GetLoopTimes))))
        (bind _returnvalue (UserInterface|CreateWidget "/Game/FlashEffect/W_FlashEffect.W_FlashEffect_C"))
        (UserInterface|Viewport|AddtoViewport _returnvalue 0)
        (bind _result (Math|Integer|DecrementInt (Variables|Components|GetLoopTimes))
          (:%20%20
            (Variables|Components|SetLoopTimes _result)
            (goto _label)))
        (else
          (bind _outactors (Actor|GetAllActorsOfClass "/Game/MantaRays/BP_MantaRay.BP_MantaRay_C"))
          (for _array_element _outactors
            (Variables|/Game/MantaRays/BP_MantaRay.BP_MantaRay_C|SetSpline%20Speed _array_element (* (Variables|/Game/MantaRays/BP_MantaRay.BP_MantaRay_C|GetSpline%20Speed _array_element) _speedupfactor))
            (Components|Timeline|SetPlayRate (Variables|/Game/MantaRays/BP_MantaRay.BP_MantaRay_C|GetManta _array_element) (* (Components|Animation|GetPlayRate (Variables|/Game/MantaRays/BP_MantaRay.BP_MantaRay_C|GetManta _array_element)) _speedupfactor))))))))

(fn ConstructionScript)