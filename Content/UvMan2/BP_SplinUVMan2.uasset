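; BP_SplinUVMan2 is an actor that moves the UVMan skeletal mesh component along its spline.
; Each Tick advances a stored distance by delta time times a speed variable.
; It then sets the mesh's relative transform from the spline's local transform at that distance, turning yaw by -90 degrees and keeping the existing scale.
; The distance has no wrap or reset, and BeginPlay, overlap and the construction script do nothing.
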(event EventBeginPlay)

(event Collision|EventActorBeginOverlap
  (params (OtherActor :type Actor%20Object%20Reference)))

(event EventTick
  (params (DeltaSeconds :type Float%20%28single-precision%29))
  (Variables|Default|SetDistance%20Along%20Spline%20UVMan2 (+ (* DeltaSeconds (Variables|Default|GetSplineSpeedUVMan2)) (Variables|Default|GetDistance%20Along%20Spline%20UVMan2)))
  (Transformation|SetRelativeTransform (Variables|Default|GetUVManSkeletalSpline) (Math|Transform|MakeTransform (Math|Vector|MakeVector (.x (.location (Spline|GetTransformatDistanceAlongSpline (Variables|Default|GetSpline) (Variables|Default|GetDistance%20Along%20Spline%20UVMan2) "Local" false))) (.y (.location (Spline|GetTransformatDistanceAlongSpline (Variables|Default|GetSpline) (Variables|Default|GetDistance%20Along%20Spline%20UVMan2) "Local" false))) (+ (.z (.location (Spline|GetTransformatDistanceAlongSpline (Variables|Default|GetSpline) (Variables|Default|GetDistance%20Along%20Spline%20UVMan2) "Local" false))) 0.0)) (Math|Rotator|MakeRotator (.roll (.rotation (Spline|GetTransformatDistanceAlongSpline (Variables|Default|GetSpline) (Variables|Default|GetDistance%20Along%20Spline%20UVMan2) "Local" false))) (.pitch (.rotation (Spline|GetTransformatDistanceAlongSpline (Variables|Default|GetSpline) (Variables|Default|GetDistance%20Along%20Spline%20UVMan2) "Local" false))) (+ (.yaw (.rotation (Spline|GetTransformatDistanceAlongSpline (Variables|Default|GetSpline) (Variables|Default|GetDistance%20Along%20Spline%20UVMan2) "Local" false))) -9e+01)) (Variables|/Script/Engine.SceneComponent|GetRelativeScale3D (Variables|Default|GetUVManSkeletalSpline))) false false))

(fn ConstructionScript)