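; BP_MantaRay is a manta ray actor that loops continuously along a referenced spline.
; Tick advances the distance by SplineSpeed and sets the actor's position, pitch and yaw from the spline, with roll driven by a Timeline.
; Reaching spline points listed in AnimationArray plays that Timeline for a full barrel roll.
; It also starts a DoOnce-guarded, LoopTimes-counted sequence of delayed screen flash widgets.
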(event Collision|EventActorBeginOverlap
  (params (OtherActor :type Actor%20Object%20Reference)))

(event EventTick
  (params (DeltaSeconds :type Float%20%28single-precision%29))
  (bind _spline (Variables|Default|GetSpline))
  (bind _spline_2 (Variables|/Game/SplineFolder/SplinePathBP.SplinePathBP_C|GetSpline _spline))
  (Utilities|FlowControl|Sequence
    (:then_0
      (Variables|Default|SetDistance%20Along%20Spline (+ (* DeltaSeconds (Variables|Default|GetSpline%20Speed)) (Variables|Default|GetDistance%20Along%20Spline))))
    (:then_1
      (for _array_element (Variables|Default|GetAnimationArray)
        (if (Utilities|Operators|EqualEqual (Spline|GetLocationatSplinePoint (Variables|/Game/SplineFolder/SplinePathBP.SplinePathBP_C|GetSpline (Variables|Default|GetSpline)) _array_element "World") (Transformation|GetActorLocation) 1.0)
          (Utilities|FlowControl|Sequence
            (:then_0
              ;[1 1 1] 5 Flashes
              (Utilities|FlowControl|DoOnce false :!label _label
                (:Completed
                  (if (> (Variables|Default|GetLoopTimes) 0) :!label _label_2
                    (Utilities|FlowControl|Delay (Utilities|Array|Get(acopy) (Variables|Default|GetDuration) (- 5 (Variables|Default|GetLoopTimes))))
                    (bind _returnvalue (UserInterface|CreateWidget "/Game/FlashEffect/W_FlashEffect.W_FlashEffect_C"))
                    (UserInterface|Viewport|AddtoViewport _returnvalue 0)
                    (bind _result (Math|Integer|DecrementInt (Variables|Default|GetLoopTimes))
                      (:%20%20
                        (Variables|Default|SetLoopTimes _result)
                        (goto _label_2)))
                    (else
                      (goto _label Reset))))))
            (:then_1
              (bind _newtrack_0 (Timeline|Timeline Play)
                (:Update
                  _)))))
        (Transformation|SetActorTransform (Math|Transform|MakeTransform (Spline|GetLocationatDistanceAlongSpline _spline_2 (Variables|Default|GetDistance%20Along%20Spline) "World") (Math|Rotator|MakeRotator (+ (Math|Float|Lerp 0.0 3.6e+02 _newtrack_0) 0.0) (.Pitch (Math|Rotator|BreakRotator (Spline|GetRotationatDistanceAlongSpline _spline_2 (Variables|Default|GetDistance%20Along%20Spline) "World"))) (.Yaw (Math|Rotator|BreakRotator (Spline|GetRotationatDistanceAlongSpline _spline_2 (Variables|Default|GetDistance%20Along%20Spline) "World"))))))
        (Utilities|FlowControl|Sequence
          (:then_0
            ;[1 1 1] Loop
            (if (>= (Variables|Default|GetDistance%20Along%20Spline) (Spline|GetSplineLength (Variables|/Game/SplineFolder/SplinePathBP.SplinePathBP_C|GetSpline (Variables|Default|GetSpline))))
              (Variables|Default|SetDistance%20Along%20Spline 0.0))))))))

(fn ConstructionScript)